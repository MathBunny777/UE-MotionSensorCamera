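; Player Blueprint that drives the camera from rotation data read over a serial COM port.
; BeginPlay opens the port, enables input and adds the first-person Enhanced Input mapping context.
; Each Tick, successfully processed serial readings are printed and fed into controller yaw, pitch and roll, with axes remapped and pitch and roll inverted.
; A reset-camera action zeroes the serial data, and EndPlay closes the port.
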(event Input|EnhancedActionEvents|EnhancedInputActionIA_ResetCamera
  (params (ActionValue :type Boolean) (ElapsedSeconds :type Float%20%28double-precision%29) (TriggeredSeconds :type Float%20%28double-precision%29) (InputAction :type Input%20Action%20Object%20Reference :default "/Game/Inputs/IA_ResetCamera.IA_ResetCamera"))
  ;[0.15 0.15 0.15 0.5] Reset Camera
  (Class|ReadSerialMotSensorLibrary|ZeroSerialData))

(event EventBeginPlay
  ;[0.15 0.15 0.15 0.5] Initialization
  (Utilities|FlowControl|Sequence
    (:then_0
      (bind (_bopened _returnvalue) (Class|ComSerial|OpenComPort 4 9600))
      (if _bopened
        (Utilities|FlowControl|Sequence
          (:then_0
            (bind _output_get (Variables|Default|SetMy%20Serial%20Port _returnvalue))
            (Class|ComSerial|Flush _output_get)
            (Class|ComSerial|Print _output_get "PORT is INITIALIZED")
            (Development|PrintString "PORT is INITIALIZED"))
          (:then_1
            (Input|EnableInput (Game|GetPlayerController 0))))
        (else
          (Development|PrintString "Port Not Opened"))))
    (:then_1
      (bind _asplayer_controller (Utilities|Casting|CastToPlayerController (Game|GetPlayerController 0)))
      (Utilities|IsValid (PlayerController|LocalPlayerSubsystems|GetEnhancedInputLocalPlayerSubsystem _asplayer_controller)
        (:Is%20Valid
          (Input|AddMappingContext (PlayerController|LocalPlayerSubsystems|GetEnhancedInputLocalPlayerSubsystem _asplayer_controller) "/Game/Inputs/IMC_FP.IMC_FP" 0 "(bIgnoreAllPressedKeysUntilRelease=True,bForceImmediately=False,bNotifyUserSettings=False)"))))))

(event Collision|EventActorBeginOverlap
  (params (OtherActor :type Actor%20Object%20Reference)))

(event EventTick
  (params (DeltaSeconds :type Float%20%28single-precision%29))
  ;[0.15 0.15 0.15 0.5] Camera Control
  (bind (_success _rx _ry _rz _returnvalue) (Class|ReadSerialMotSensorLibrary|ProcessSerialData))
  (if _success
    (Utilities|FlowControl|Sequence
      (:then_0
        (Development|PrintString _returnvalue))
      (:then_1
        (Pawn|Input|AddControllerYawInput _rx)
        (Pawn|Input|AddControllerPitchInput (* _rz -1.0))
        (Pawn|Input|AddControllerRollInput (* _ry -1.0))))))

(event EventEndPlay
  (params (EndPlayReason :type EEndPlayReason%20Enum :default "Destroyed"))
  (bind _my_serial_port (Variables|Default|GetMy%20Serial%20Port))
  ;[0.15 0.15 0.15 0.5] Clean up
  (Class|ComSerial|Println _my_serial_port "Program Is Terminated")
  (Class|ComSerial|Close _my_serial_port))

(fn ConstructionScript)